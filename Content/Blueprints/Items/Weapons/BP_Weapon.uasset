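; BP_Weapon is a weapon item Blueprint that detects hits with a box trace.
; When WeaponBox begins overlapping, it traces a small box on the Visibility channel between Start and End component locations.
; The trace and a sphere at the impact point are drawn for debugging, with no damage applied here.
; Sphere overlap does nothing, and leftover bobbing and hand-socket attachment nodes are disconnected.
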(event `self.ReceiveTick`
  (params (DeltaSeconds :type "Float (single-precision)")))

(event `self.Sphere.OnComponentBeginOverlap`
  (params (OverlappedComponent :type "PrimitiveComponent Object Reference") (OtherActor :type "Actor Object Reference") (OtherComp :type "PrimitiveComponent Object Reference") (OtherBodyIndex :type Integer) (bFromSweep :type Boolean) (SweepResult :type "HitResult Structure (by ref)")))

(event `self.WeaponBox.OnComponentBeginOverlap`
  (params (OverlappedComponent :type "PrimitiveComponent Object Reference") (OtherActor :type "Actor Object Reference") (OtherComp :type "PrimitiveComponent Object Reference") (OtherBodyIndex :type Integer) (bFromSweep :type Boolean) (SweepResult :type "HitResult Structure (by ref)"))
  (bind _outhit (`KismetSystemLibrary.BoxTraceSingle` :`Start` (`SceneComponent.K2_GetComponentLocation` (`self.Start`)) :`End` (`SceneComponent.K2_GetComponentLocation` (`self.End`)) :`HalfSize` (2.5 2.5 2.5) :`TraceChannel` "TraceTypeQuery1" :`DrawDebugType` "ForDuration"))
  (`KismetSystemLibrary.DrawDebugSphere` (`.ImpactPoint` (`GameplayStatics.BreakHitResult` _outhit)) 25.0 12 (struct :`G` 0.020531 :`B` 1.0 :`A` 1.0) 5.0))

(fn `UserConstructionScript`)